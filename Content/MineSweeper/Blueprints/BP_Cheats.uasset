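; BP_Cheats provides cheat events for the Minesweeper game: opening a cell, resetting the game and revealing mines.
; Each event casts player controller 0 to TopDownController and delegates the work to it.
; OpenCell fetches the block at the given X and Y, uncovers it, then calls Win if the controller's MineLeft count is zero.
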(event EventOpenCell
  (params (x :type Integer) (y :type Integer))
  (bind _astop_down_controller (Utilities|Casting|CastToTopDownController (Game|GetPlayerController 0)))
  (bind _block (Default|GetBlock _astop_down_controller x y))
  (Default|Uncover _block)
  (if (== (Variables|/Game/MineSweeper/Blueprints/TopDownController.TopDownController_C|GetMineLeft _astop_down_controller) 0)
    (Default|Win _astop_down_controller)))

(event EventReset
  (bind _astop_down_controller (Utilities|Casting|CastToTopDownController (Game|GetPlayerController 0)))
  (Default|ResetGame _astop_down_controller))

(event EventShowMines
  (bind _astop_down_controller (Utilities|Casting|CastToTopDownController (Game|GetPlayerController 0)))
  (Default|ViewMine _astop_down_controller))